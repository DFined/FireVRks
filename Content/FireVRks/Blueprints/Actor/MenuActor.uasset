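; VR menu actor that enables player input, adds the menu input mapping context and shows a cursor where the player points.
; On BeginPlay it caches the pawn's left and right Widget Interaction components by pointer index, plus the right-aim motion controller.
; Each Tick moves the cursor to the right interaction component's last hit location.
; Missing pawn components only print a warning.
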(event EventBeginPlay
  (Input|EnableInput (Game|GetPlayerController 0))
  (Input|AddMappingContext (PlayerController|LocalPlayerSubsystems|GetEnhancedInputLocalPlayerSubsystem (Game|GetPlayerController 0)) "/Game/FireVRks/Input/IMC_Menu.IMC_Menu" 3 "(bIgnoreAllPressedKeysUntilRelease=True,bForceImmediately=False)")
  (CallFunction|SetWidgetInteractionReferences)
  (CallFunction|SetMotionControllerReference))

(event Collision|EventActorBeginOverlap
  (params (OtherActor :type Actor%20Object%20Reference)))

(event EventTick
  (params (DeltaSeconds :type Float%20%28single-precision%29))
  (Transformation|SetWorldLocation (Variables|Default|GetCursor) (.Location (Collision|BreakHitResult (Class|WidgetInteractionComponent|GetLastHitResult (Variables|Default|GetWidget%20Interaction%20Ref%20Right)))) false false))

(fn ConstructionScript)

(fn SetWidgetInteractionReferences
  (bind _returnvalue (Game|Player|GetPlayerPawn 0))
  (bind _returnvalue_2 (Actor|GetComponentsByClass _returnvalue "/Script/UMG.WidgetInteractionComponent"))
  (if (> (Utilities|Array|Length _returnvalue_2) 0) ; Are there any Widget Interaction Components attached to the Player Pawn?
    (bind _output_get (LocalVariables|SetLocalWidgetInteractionComponents _returnvalue_2))
    (for _array_element _output_get ; Get the Pawn's Widget Interaction Components
      (if (== (Variables|/Script/UMG.WidgetInteractionComponent|GetPointerIndex _array_element) 0) ; Pointer Index 0 is assigned to the Left WIC
        (Variables|Default|SetWidget%20Interaction%20Ref%20Left _array_element)
        (else
          (Variables|Default|SetWidget%20Interaction%20Ref%20Right _array_element))))
    (else
      (Development|PrintString "Warning: No WidgetInteractionComponent was found. Menu interaction will FAIL"))))

(fn SetMotionControllerReference
  (bind _returnvalue (Game|Player|GetPlayerPawn 0))
  (bind _returnvalue_2 (Actor|GetComponentsByClass _returnvalue "/Script/HeadMountedDisplay.MotionControllerComponent"))
  (if (> (Utilities|Array|Length _returnvalue_2) 0) ; Are there any Motion Controllers attached to the Player Pawn?
    (bind _output_get (LocalVariables|SetLocalMotionControllers _returnvalue_2))
    (for _array_element _output_get
      (if (Utilities|Name|Equal(Name) (Variables|/Script/HeadMountedDisplay.MotionControllerComponent|GetMotionSource _array_element) (select true "RightAim" "LeftAim"))
        (Variables|Default|SetMotionController _array_element)))
    (else
      (Development|PrintString "Warning: No WidgetInteractionComponent was found. Menu interaction will FAIL"))))