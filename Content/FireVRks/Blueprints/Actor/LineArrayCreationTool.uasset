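; Placement tool actor that previews an evenly spaced line of ghost markers, then replaces them with spawned actors.
; SetNumIntermediates rebuilds translucent, collision-free ghost meshes under Pos1Marker.
; SetPos2 moves the end marker and lerps those meshes from the actor's location to that point.
; Finalize spawns the given class at each ghost, oriented along the line, then destroys the tool and returns the spawned actors.
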(event EventBeginPlay)

(event Collision|EventActorBeginOverlap
  (params (OtherActor :type Actor%20Object%20Reference)))

(event EventTick
  (params (DeltaSeconds :type Float%20%28single-precision%29)))

(fn ConstructionScript)

(fn SetPos2
  (params (Pos2 :type Vector))
  (bind _pos1marker (Variables|Default|GetPos1Marker))
  (bind _children (Components|GetChildrenComponents _pos1marker false))
  (bind _output_get (Variables|Default|SetPos2 Pos2))
  (Transformation|SetWorldLocation (Variables|Default|GetPos2Marker) _output_get false false)
  (for (_array_element _array_index) _children
    (Transformation|SetWorldLocation _array_element (Math|Vector|Lerp(Vector) (Transformation|GetActorLocation) (Variables|Default|GetPos2) (/ _array_index (+ (Utilities|Array|Length _children) -1))) false false)))

(fn SetNumIntermediates
  (params (NumIntermediates :type Integer))
  (bind _output_get (Variables|Default|SetNumIntermediates NumIntermediates))
  (for _array_element (Components|GetChildrenComponents (Variables|Default|GetPos1Marker) false)
    (Components|DestroyComponent _array_element))
  (for _index (range 0 (- _output_get 1))
    (bind _returnvalue (Game|AddComponentbyClass "/Game/FireVRks/Blueprints/Component/PrimitiveGhostMeshComponent.PrimitiveGhostMeshComponent_C" false (Math|Transform|MakeTransform "0, 0, 0" "0, 0, 0" "0.300000,0.300000,0.300000") (Math|Color|MakeColor 0.5 0.7 0.1 0.02)))
    (Collision|SetCollisionEnabled _returnvalue "NoCollision")
    (Transformation|AttachComponentToComponent _returnvalue (Variables|Default|GetPos1Marker) "None" "KeepRelative" "KeepRelative" "KeepRelative" true)))

(fn Finalize
  (params (Class :type Actor%20Class%20Reference))
  (bind _tmparray (Variables|Default|GetTmpArray))
  (Utilities|Array|Clear _tmparray)
  (for _array_element (Components|GetChildrenComponents (Variables|Default|GetPos1Marker) false)
    (bind _returnvalue (Game|SpawnActorfromClass Class (Math|Transform|MakeTransform (Transformation|GetWorldLocation _array_element) (Math|Conversions|RotationFromXVector (- (Transformation|GetWorldLocation (Variables|Default|GetPos2Marker)) (Transformation|GetWorldLocation (Variables|Default|GetPos1Marker))))) "Undefined" "MultiplyWithRoot" 0 0))
    (Utilities|Array|Add _tmparray _returnvalue))
  (Actor|DestroyActor)
  (return _tmparray))